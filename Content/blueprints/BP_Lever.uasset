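; BP_Lever is a clickable lever that swings up and back to knock the player's marble, with power set by the marble's charge.
; A Tick-driven state machine lerps pitch over elapsed time, bouncing marbles hit on the forward swing along the impact normal.
; A push-out box shrinks by cosine as it rotates, and a kick-out box, active at rest, relocates non-swept marble overlaps.
; Cursor hover updates the HUD's interaction count.
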(event `self.ReceiveTick`
  (params (DeltaSeconds :type "Float (single-precision)"))
  (switch `/Game/blueprints/ELeverState` (`self.State`)
    (:`NewEnumerator1`
      (`self.Swing Forward Update`))
    (:`NewEnumerator2`
      (`self.Swing Backward Update`))))

(event `self.ClickCapsule.OnReleased`
  (params (TouchedComponent :type "PrimitiveComponent Object Reference") (ButtonReleased :type "Key Structure"))
  (if (== ButtonReleased "LeftMouseButton")
    (`self.Start Swing`)))

(event `self.ClickCapsule.OnBeginCursorOver`
  (params (TouchedComponent :type "PrimitiveComponent Object Reference"))
  (`self.Begin Cursor Hover`))

(event `self.ClickCapsule.OnEndCursorOver`
  (params (TouchedComponent :type "PrimitiveComponent Object Reference"))
  (`self.End Cursor Hover`))

(event `self.KickOutBox.OnComponentBeginOverlap`
  (params (OverlappedComponent :type "PrimitiveComponent Object Reference") (OtherActor :type "Actor Object Reference") (OtherComp :type "PrimitiveComponent Object Reference") (OtherBodyIndex :type Integer) (bFromSweep :type Boolean) (SweepResult :type "HitResult Structure (by ref)"))
  (`self.Kick Out Marble` OtherActor bFromSweep))

(event `self.Lever.OnComponentHit`
  (params (HitComponent :type "PrimitiveComponent Object Reference") (OtherActor :type "Actor Object Reference") (OtherComp :type "PrimitiveComponent Object Reference") (NormalImpulse :type "Vector Structure") (Hit :type "HitResult Structure (by ref)"))
  (`self.Swing Impulse` OtherActor NormalImpulse))

(fn `Begin Cursor Hover`
  (bind _asbp_marble_controller (cast `/Game/blueprints/BP_MarbleController` (`GameplayStatics.GetPlayerController` 0)))
  (bind _hud (`/Game/blueprints/BP_MarbleController.Get HUD` _asbp_marble_controller))
  (`/Game/ui/WBP_HUD.Increment Interactions` _hud))

(fn `Calc Swing Factor`
  (returns (`Return Value` :type "Float (double-precision)"))
  (return (/ (* (`self.Swing Speed`) (- (`KismetSystemLibrary.GetGameTimeInSeconds`) (`self.Swing Start Time`)) (`self.Rotation Damping`)) (/ (`self.Swing Angle`) 90.0))))

(fn `End Cursor Hover`
  (bind _asbp_marble_controller (cast `/Game/blueprints/BP_MarbleController` (`GameplayStatics.GetPlayerController` 0)))
  (bind _hud (`/Game/blueprints/BP_MarbleController.Get HUD` _asbp_marble_controller))
  (`/Game/ui/WBP_HUD.Decrement Interactions` _hud))

(fn `Kick Out Marble`
  (params (Actor :type "Object Object Reference") (`From Sweep` :type Boolean))
  (bind _asbp_marble (cast `/Game/blueprints/BP_Marble` Actor))
  (if (not `From Sweep`)
    (`/Game/blueprints/BP_Marble.Override World Location` _asbp_marble (`SceneComponent.K2_GetComponentLocation` (`self.KickOutLocation`)))))

(fn `Set Swing Rotation`
  (params (Angle :type "Float (double-precision)"))
  (bind _returnvalue (`KismetMathLibrary.FClamp` Angle 0.0 (`self.Swing Angle`)))
  (`SceneComponent.K2_SetRelativeRotation` (`self.LeverRotator`) (`KismetMathLibrary.MakeRotator` 0.0 _returnvalue) false false)
  (`SceneComponent.SetRelativeScale3D` (`self.PushOutBoxScalar`) (`KismetMathLibrary.MakeVector` (`KismetMathLibrary.DegCos` (/ (* _returnvalue 90.0) (`self.Swing Angle`))) 1.0 1.0)))

(fn `Start Swing`
  (if (`|EnumEquality` (`self.State`) "NewEnumerator0")
    (bind _asbp_marble (cast `/Game/blueprints/BP_Marble` (`GameplayStatics.GetPlayerPawn` 0)))
    (set `self.Swing Speed` (`KismetMathLibrary.Lerp` (`self.Swing Min Power`) (`self.Swing Max Power`) (`/Game/blueprints/BP_Marble.Get Charge Factor` _asbp_marble)))
    (`/Game/blueprints/BP_Marble.Reset Charge Time` _asbp_marble)
    (set `self.Swing Start Time` (`KismetSystemLibrary.GetGameTimeInSeconds`))
    (set `self.State` "NewEnumerator1")
    (`PrimitiveComponent.SetCollisionEnabled` (`self.KickOutBox`) "NoCollision")))

(fn `Swing Backward Update`
  (bind _returnvalue (`KismetMathLibrary.Lerp` (`self.Swing Angle`) 0.0 (`self.Calc Swing Factor`)))
  (`self.Set Swing Rotation` _returnvalue)
  (if (<= _returnvalue 0.0)
    (set `self.State` "NewEnumerator0")
    (`PrimitiveComponent.SetCollisionEnabled` (`self.KickOutBox`) "QueryOnly")))

(fn `Swing Forward Update`
  (bind _swing_angle (`self.Swing Angle`))
  (bind _returnvalue (`KismetMathLibrary.Lerp` 0.0 _swing_angle (`self.Calc Swing Factor`)))
  (`self.Set Swing Rotation` _returnvalue)
  (if (>= _returnvalue _swing_angle)
    (set `self.Swing Start Time` (`KismetSystemLibrary.GetGameTimeInSeconds`))
    (set `self.State` "NewEnumerator2")))

(fn `Swing Impulse`
  (params (Actor :type "Actor Object Reference") (`Normal Impulse` :type "Vector Structure"))
  (bind _asbp_marble (cast `/Game/blueprints/BP_Marble` Actor))
  (if (`|EnumEquality` (`self.State`) "NewEnumerator1")
    (`/Game/blueprints/BP_Marble.Bounce` _asbp_marble (* (`KismetMathLibrary.Normal` `Normal Impulse`) (`self.Swing Speed`)))))

(fn `UserConstructionScript`)