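; BP_Ring is a spinning, numbered collectible ring that the marble picks up on a pinball machine.
; Construction shows only the child number mesh whose name contains "Num_" plus the ring's Number.
; A BP_Marble overlap passes that Number to the parent BP_PinballMachine's CollectRing, which decides whether the pickup succeeds.
; Success hides the ring and number and disables sphere collision; Uncollect restores them.
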(event `self.ReceiveTick`
  (params (DeltaSeconds :type "Float (single-precision)"))
  (`self.Spin` DeltaSeconds))

(event `self.Sphere.OnComponentBeginOverlap`
  (params (OverlappedComponent :type "PrimitiveComponent Object Reference") (OtherActor :type "Actor Object Reference") (OtherComp :type "PrimitiveComponent Object Reference") (OtherBodyIndex :type Integer) (bFromSweep :type Boolean) (SweepResult :type "HitResult Structure (by ref)"))
  (cast `/Game/blueprints/BP_Marble` OtherActor)
  (`self.Collect`))

(fn `Collect`
  (bind _asbp_pinball_machine (cast `/Game/blueprints/BP_PinballMachine` (`self.GetAttachParentActor`)))
  (bind _success (`/Game/blueprints/BP_PinballMachine.Collect Ring` _asbp_pinball_machine (`self.#Number`)))
  (if _success
    (`self.Hide` true)))

(fn `Determine Num Mesh`
  (for _array_element (`SceneComponent.GetChildrenComponents` (`self.Nums`) false)
    (bind _asstatic_mesh_component (cast `StaticMeshComponent` _array_element))
    (bind _returnvalue (`self.Mesh Is Corresponding #Number` _asstatic_mesh_component))
    (`SceneComponent.SetHiddenInGame` _asstatic_mesh_component (not _returnvalue) false)
    (`SceneComponent.SetVisibility` _asstatic_mesh_component _returnvalue false)
    (if _returnvalue
      (set `self.NumMesh` _asstatic_mesh_component))))

(fn `Hide`
  (params (Hide :type Boolean))
  (bind _nummesh (`self.NumMesh`))
  (`/Engine/EditorBlueprintResources/StandardMacros.IsValid` self
    (:`Is Valid`
      (`SceneComponent.SetHiddenInGame` (`self.Ring`) Hide false)
      (`PrimitiveComponent.SetCollisionEnabled` (`self.Sphere`) (select `bool` Hide :`false` "QueryOnly" :`true` "NoCollision" :!type "ECollisionEnabled Enum"))
      (`/Engine/EditorBlueprintResources/StandardMacros.IsValid` _nummesh
        (:`Is Valid`
          (`SceneComponent.SetHiddenInGame` _nummesh Hide false))))))

(fn `Mesh Is Corresponding #Number`
  (params (Object :type "Object Object Reference"))
  (returns (ReturnValue :type Boolean))
  (return (!= (`KismetStringLibrary.FindSubstring` (`KismetSystemLibrary.GetDisplayName` Object) (`KismetStringLibrary.Concat_StrStr` "Num_" (`KismetStringLibrary.Conv_IntToString` (`self.#Number`)))) -1)))

(fn `Spin`
  (params (`Delta Time` :type "Float (double-precision)"))
  (bind _ring (`self.Ring`))
  (bind (_relativerotation_roll _relativerotation_pitch _relativerotation_yaw) (`KismetMathLibrary.BreakRotator` (`SceneComponent.RelativeRotation` _ring)))
  (`SceneComponent.K2_SetRelativeRotation` _ring (`KismetMathLibrary.MakeRotator` _relativerotation_roll _relativerotation_pitch (+ _relativerotation_yaw (* `Delta Time` (`self.Spin Speed`)))) false false))

(fn `Uncollect`
  (`self.Hide` false))

(fn `UserConstructionScript`
  (`self.Determine Num Mesh`))