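; BP_PinballSurface is a surface actor that detects the player's marble and reports its own orientation and normal.
; Every tick it tests the box components under StickVolumes for physics-body overlaps with the player BP_Marble's static mesh, setting OverlappingMarble on the first match.
; Helper functions return the actor rotation as the surface orientation and world up rotated by it as the surface normal.
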(event `self.ReceiveTick`
  (params (DeltaSeconds :type "Float (single-precision)"))
  (`self.Check For Marble Overlap`))

(fn `Check For Marble Overlap`
  (bind _children (`SceneComponent.GetChildrenComponents` (`self.Stick Volumes`) false))
  (set `self.Overlapping Marble` false)
  (bind _asbp_marble (cast `/Game/blueprints/BP_Marble` (`GameplayStatics.GetPlayerPawn` 0)))
  (for _index (range (`KismetArrayLibrary.Array_Length` _children))
    (bind _asbox_collision (cast `BoxComponent` (`|GetArrayItem` _children _index)))
    (bind _staticmesh (`/Game/blueprints/BP_Marble.StaticMesh` _asbp_marble))
    (bind _outcomponents (`KismetSystemLibrary.ComponentOverlapComponents` _asbox_collision (`SceneComponent.K2_GetComponentToWorld` _asbox_collision) (`|MakeArray` "ObjectTypeQuery4" :!type "EObjectTypeQuery Enum") (`GameplayStatics.GetObjectClass` _staticmesh)))
    (if (`KismetArrayLibrary.Array_Contains` _outcomponents _staticmesh)
      (set `self.Overlapping Marble` true)
      (break))))

(fn `Get Surface Normal`
  (returns (Normal :type "Vector Structure"))
  (return (`KismetMathLibrary.GreaterGreater_VectorRotator` (`KismetMathLibrary.MakeVector` 0.0 0.0 1.0) (`self.Get Surface Orientation`))))

(fn `Get Surface Orientation`
  (returns (Orientation :type "Rotator Structure"))
  (return (`self.K2_GetActorRotation`)))

(fn `UserConstructionScript`)