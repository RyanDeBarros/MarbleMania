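; Pinball machine puzzle that captures the player's marble, holds exit gates shut until all attached coins are removed, and completes once the marble leaves.
; Tick drives capture states: touching a sticky volume enables invisible walls, and staying in an exit volume past a wait time completes it.
; Walls, gates and volumes are child components of containers, walked by loop macros that poll marble overlaps.
; It exposes StickyMarble state and a rotation-derived surface normal.
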(event `self.ReceiveBeginPlay`
  (`self.Setup Initial Coins`)
  (`self.Check For Exit Gate Unlock`))

(event `self.ReceiveTick`
  (params (DeltaSeconds :type "Float (single-precision)"))
  (switch `/Game/blueprints/EPinballMarbleCaptureState` (`self.Marble Capture State`)
    (:`NewEnumerator0`
      (`self.Tick - Pre-Captured Marble`))
    (:`NewEnumerator1`
      (`self.Tick - Captured Marble` DeltaSeconds))))

(fn `Check For Exit Gate Unlock`
  (if (`KismetArrayLibrary.Array_IsEmpty` (`self.Coins`))
    (bind _static_mesh (`self.Loop Over Static Meshes` (`self.Exit Gates`))
      (:`Loop Body`
        (`PrimitiveComponent.SetCollisionEnabled` _static_mesh "NoCollision")
        (`SceneComponent.SetHiddenInGame` _static_mesh true true)))))

(fn `Check For Exiting Marble`
  (`self.Check For Ovelapping Marble` (`self.Exit Volumes`) (`self.Exiting Marble`)))

(fn `Check For Ovelapping Marble`
  (params (Volumes :type "SceneComponent Object Reference") (Overlapping :type "Boolean (by ref)"))
  (`|VariableSetRef` Overlapping)
  (`self.Loop Over Volumes` Volumes :!label _label
    (:`Loop Body`
      (`|VariableSetRef` Overlapping true)
      (goto _label :!via `Break`))
    (:`Completed`
      (return))))

(fn `Check For Sticky Marble`
  (`self.Check For Ovelapping Marble` (`self.Sticky Volumes`) (`self.Sticky Marble`)))

(fn `Get Surface Normal`
  (returns (Normal :type "Vector Structure"))
  (return (`KismetMathLibrary.GreaterGreater_VectorRotator` (`KismetMathLibrary.MakeVector` 0.0 0.0 1.0) (`self.Get Surface Orientation`))))

(fn `Get Surface Orientation`
  (returns (Orientation :type "Rotator Structure"))
  (return (`self.K2_GetActorRotation`)))

(fn `Remove Coin`
  (params (Coin :type "/Game/blueprints/BP_Coin Object Reference"))
  (`KismetArrayLibrary.Array_RemoveItem` (`self.Coins`) Coin)
  (`self.Check For Exit Gate Unlock`))

(fn `Setup Initial Coins`
  (for _array_element (`self.GetAttachedActors` true true)
    (bind _asbp_coin (cast `/Game/blueprints/BP_Coin` _array_element))
    (`KismetArrayLibrary.Array_Add` (`self.Coins`) _asbp_coin)))

(fn `Setup Initial Invisible Walls`
  (bind _static_mesh (`self.Loop Over Static Meshes` (`self.Invisible Walls`))
    (:`Loop Body`
      (`PrimitiveComponent.SetMaterial` _static_mesh 0 "/Game/materials/M_Invisible.M_Invisible")
      (`PrimitiveComponent.SetCollisionEnabled` _static_mesh "NoCollision"))))

(fn `Tick - Captured Marble`
  (params (`Delta Time` :type "Float (double-precision)"))
  (`self.Check For Exiting Marble`)
  (`self.Update Exit Wait Time` `Delta Time`
    (:`Full Exit`
      (set `self.Sticky Marble` false)
      (set `self.Marble Capture State` "NewEnumerator2"))
    (:`Still Sticky`
      (`self.Check For Sticky Marble`))))

(fn `Tick - Pre-Captured Marble`
  (`self.Check For Sticky Marble`)
  (if (`self.Sticky Marble`)
    (set `self.Marble Capture State` "NewEnumerator1")
    (bind _static_mesh (`self.Loop Over Static Meshes` (`self.Invisible Walls`))
      (:`Loop Body`
        (`PrimitiveComponent.SetCollisionEnabled` _static_mesh "PhysicsOnly")))))

(fn `UserConstructionScript`
  (`self.Setup Initial Invisible Walls`))